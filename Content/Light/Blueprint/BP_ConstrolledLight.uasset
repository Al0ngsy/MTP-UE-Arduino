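; Point light actor that the player toggles on and off with the D key, fading smoothly between dark and a maximum intensity.
; Each Tick applies the current intensity, ramps it toward the IsLightOn target at one clamped, delta-time-scaled rate, then polls the key.
; Input is polled on a PlayerController cached at BeginPlay, and each press prints a millisecond UTC timestamp before flipping the state.
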(event `self.ReceiveBeginPlay`
  (bind _returnvalue (`InputDeviceLibrary.GetPlayerControllerFromInputDevice` (struct)))
  (set `self.PlayerController` _returnvalue))

(event `self.ReceiveTick`
  (params (DeltaSeconds :type "Float (single-precision)"))
  (bind _intensityincreaseratepersecond (`self.IntensityIncreaseRatePerSecond`))
  (set `self.Delta Seconds` DeltaSeconds)
  (`|ExecutionSequence`
    (:`then_1`
      (`LightComponent.SetIntensity` (`self.PointLight`) (`self.Intensity`)))
    (:`then_2`
      (if (`self.IsLightOn`)
        (if (<= (`self.Intensity`) (`self.MaxIntensity`))
          (set `self.Intensity` (`KismetMathLibrary.FClamp` (+ (* (`self.Delta Seconds`) _intensityincreaseratepersecond) (`self.Intensity`)) 0.0 (`self.MaxIntensity`))))
        (elif (>= (`self.Intensity`) 0.0)
          (set `self.Intensity` (`KismetMathLibrary.FClamp` (- (`self.Intensity`) (* _intensityincreaseratepersecond (`self.Delta Seconds`))) 0.0 (`self.MaxIntensity`))))))
    (:`then_3`
      (`|ExecutionSequence`
        (:`then_0`
          (if (`PlayerController.WasInputKeyJustPressed` (`self.PlayerController`) "D")
            (bind _time_with_text (`self.Get UTC Time` "D pressed"))
            (`KismetSystemLibrary.PrintString` (`KismetTextLibrary.Conv_TextToString` _time_with_text) true true (struct :`G` 1.0 :`A` 1.0) 4.0)
            (if (`self.IsLightOn`)
              (set `self.IsLightOn` false)
              (else
                (set `self.IsLightOn` true)))))))))

(fn `Get UTC Time`
  (params (`Text To Concat` :type Text))
  (returns (`Time with Text` :type Text))
  (bind (_year _month _day _hour _minute _second _millisecond) (`KismetMathLibrary.BreakDateTime` (`KismetMathLibrary.UtcNow`)))
  (return (`|FormatText` "UTC Time: {y}-{m}-{d}T{hh}:{min}:{s}:{ms}Z - {t}" (`KismetTextLibrary.Conv_IntToText` _year false false) _month _day _hour _minute _second _millisecond `Text To Concat`)))

(fn `UserConstructionScript`)